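; LinkLine_BP is a link line Blueprint that replays the animation of a line one link at a time.
; BeginReplayLinkAnimation walks CurrentReplayLength from 1 up to the LinkLinePoints count, printing a debug message and calling ReplaySingleLinkLineAniamtion for each index, then calls EndReplayLinkAnimation.
; The pacing comes from WhileLoopWithDealy, a local macro that builds a timed while loop by looping back through a retriggerable delay.
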(event EventBeginReplayLinkAnimation
  (Variables|Default|SetCurrentReplayLength 1)
  (Utilities|WhileLoopwithDealy (< (Variables|Default|GetCurrentReplayLength) (Utilities|Array|Length (Variables|Default|GetLinkLinePoints))) 0.2
    (:Loop%20Body
      (Development|PrintText (Utilities|Text|ToText(String) (Utilities|String|Append "Replay Link " (Utilities|String|ToString(Integer) (Variables|Default|GetCurrentReplayLength)))))
      (Class|SGLinkLine|ReplaySingleLinkLineAniamtion (Variables|Default|GetCurrentReplayLength))
      (Math|Integer|IncrementInt (Variables|Default|GetCurrentReplayLength)))
    (:Completed
      (Class|SGLinkLine|EndReplayLinkAnimation))))

(event EventBeginPlay)

(event EventActorBeginOverlap
  (params (OtherActor :type Actor%20Object%20Reference)))

(event EventTick
  (params (DeltaSeconds :type Float%20%28single-precision%29)))

(fn ConstructionScript)