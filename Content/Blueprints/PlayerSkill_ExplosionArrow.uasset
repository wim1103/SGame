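; Player skill actor that fires an explosive arrow at a random tile on the puzzle grid and collects the surrounding tiles.
; On use, it picks a random non-edge column and row from the game mode's current grid.
; It moves the arrow and explosion particle component to that tile, restarts the effect, then after a short delay collects the tile square around that position.
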(event Collision|EventActorBeginOverlap
  (params (OtherActor :type Actor%20Object%20Reference)))

(event EventTick
  (params (DeltaSeconds :type Float%20%28single-precision%29)))

(event EventPlayerUseSkill
  (bind _explosionpsc (Variables|Default|GetExplosionPSC))
  (bind _assggame_mode (Utilities|Casting|CastToSGGameMode (Game|GetGameMode)))
  (bind _output_get (Variables|Default|SetRandomColumn (Math|Random|RandomIntegerinRange 1 (- (Variables|/Script/SGame.SGGrid|GetGridWidth (Variables|/Script/SGame.SGGameMode|GetCurrentGrid _assggame_mode)) 2))))
  (bind _output_get_2 (Variables|Default|SetRandomRow (Math|Random|RandomIntegerinRange 1 (- (Variables|/Script/SGame.SGGrid|GetGridHeight (Variables|/Script/SGame.SGGameMode|GetCurrentGrid _assggame_mode)) 2))))
  (bind _returnvalue (Class|SGGrid|GetTilefromColumnandRow (Variables|/Script/SGame.SGGameMode|GetCurrentGrid _assggame_mode) _output_get _output_get_2))
  (Transformation|SetWorldLocation _explosionpsc (+ (Transformation|GetActorLocation _returnvalue) "0,20.000000, 0") false false)
  (Components|Activation|SetActive _explosionpsc true true)
  (Utilities|FlowControl|Delay 0.5)
  (bind _returnvalue_2 (Class|SGGrid|GetTileSquarefromColumnandRow (Variables|/Script/SGame.SGGameMode|GetCurrentGrid _assggame_mode) _output_get _output_get_2))
  (Class|SGGrid|CollectTileArray (Variables|/Script/SGame.SGGameMode|GetCurrentGrid _assggame_mode) _returnvalue_2))

(event EventBeginPlay)

(fn ConstructionScript)