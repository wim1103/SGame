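; Grid actor Blueprint that animates a color fade on its AttackFadingSprite when an attack fade is triggered.
; StartAttackFadeAnimation creates a linear color tween and sets IsTweening, which makes Tick copy the tween's current color onto the sprite each frame.
; The tween's completion callback, FinishAttackSpriteFading, is bound by function name and clears the flag to stop the updates.
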(event EventStartAttackFadeAnimation
  (bind _returnvalue (Class|ITween|LinearColorfromtoFull 0.0 "No Name" "(R=1.000000,G=1.000000,B=1.000000,A=1.000000)" "(R=0.000000,G=0.000000,B=0.000000,A=1.000000)" true 0.0 "first" "seconds" 5.0 "linear" 0 1.0 "once" 0 0 "" 0 "" 0 "" self "FinishAttackSpriteFading" false false))
  (Variables|Default|SetTweeningColor _returnvalue)
  (Variables|Default|SetbIsTweening true))

(event EventBeginPlay)

(event EventActorBeginOverlap
  (params (OtherActor :type Actor%20Object%20Reference)))

(event EventTick
  (params (DeltaSeconds :type Float%20%28single-precision%29))
  (if (Variables|Default|GetbIsTweening)
    (Sprite|SetSpriteColor (Variables|/Script/Paper2D.PaperSpriteActor|GetRenderComponent (Variables|Default|GetAttackFadingSprite self)) (.linearColorCurrent (Utilities|Struct|BreakDataTypeValues (Variables|/Script/SGame.iTweenEvent|Getdtv (Variables|Default|GetTweeningColor)))))))

(fn ConstructionScript)

(fn FinishAttackSpriteFading
  (Variables|Default|SetbIsTweening false))